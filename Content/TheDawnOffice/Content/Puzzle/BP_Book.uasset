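; BP_Book is an interactable puzzle book that reports its color to the level's BP_PuzzleManager when first used.
; On BeginPlay it caches the manager and the mesh's starting relative location.
; Interact fires once, registering BookColor with the manager, playing a sound and running a timeline that slides the mesh a short distance along local X.
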(event `self.ReceiveBeginPlay`
  (bind _returnvalue_location (`KismetMathLibrary.BreakTransform` (`SceneComponent.GetRelativeTransform` (`self.StaticMesh`))))
  (bind _returnvalue (`GameplayStatics.GetActorOfClass` "/Game/TheDawnOffice/Content/Puzzle/BP_PuzzleManager.BP_PuzzleManager_C"))
  (set `self.PuzzleManagerRef` _returnvalue)
  (set `self.InitialLocation` _returnvalue_location))

(event `/Game/TheDawnOffice/Content/Items/Interfaces/I_Interact.Interact`
  (params (Character :type "/Game/FirstPerson/Blueprints/BP_FirstPersonCharacter Object Reference"))
  (`/Engine/EditorBlueprintResources/StandardMacros.DoOnce` false
    (:`Completed`
      (`/Game/TheDawnOffice/Content/Puzzle/BP_PuzzleManager.RegisterBookPass` (`self.PuzzleManagerRef`) (`self.BookColor`))
      (`GameplayStatics.PlaySound2D` "/Engine/VREditor/Sounds/UI/Drop_Item_From_ContentBrowser.Drop_Item_From_ContentBrowser" 1.0 1.0 0.0 null null)
      (bind (_direction _newtrack_0) (`Timeline|Anim_PushBook`)
        (:`Update`
          (`SceneComponent.K2_SetRelativeLocation` (`self.StaticMesh`) (`KismetMathLibrary.VLerp` (`self.InitialLocation`) (+ (`self.InitialLocation`) (10.0 0.0 0.0)) _newtrack_0) false false))))))

(fn `UserConstructionScript`)