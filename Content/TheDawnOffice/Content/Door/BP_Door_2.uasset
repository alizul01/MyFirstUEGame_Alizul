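; BP_Door_2 is a lockable swinging door whose yaw animates between closed and open through timelines.
; Interact toggles it with TL_Doors, while ForceInteractDoor sets a requested state with a separate Timeline that closes by reversing from the end.
; Both ignore calls while the door is locked or moving.
; Pickup and CustomEvent each clear the lock.
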(event `self.Interact`
  (params (Character :type "/Game/FirstPerson/Blueprints/BP_FirstPersonCharacter Object Reference"))
  (if (`self.IsLocked`)
    _
    (elif (not (`self.IsMoving`))
      (set `self.IsMoving` true)
      (bind _output_get (set `self.IsOpened` (not (`self.IsOpened`))))
      (if _output_get
        (bind (_direction _door_alpha) (`Timeline|TL_Doors` :!label _label)
          (:`Update`
            (`SceneComponent.K2_SetRelativeRotation` (`self.Door`) (`KismetMathLibrary.MakeRotator` 0.0 0.0 (`KismetMathLibrary.Lerp` 0.0 100.0 _door_alpha)) false false))
          (:`Finished`
            (set `self.IsMoving` false)))
        (else
          (goto _label :!via `Reverse`))))))

(event `self.Pickup`
  (params (Doors :type "/Game/TheDawnOffice/Content/Door/BP_Door Object Reference"))
  (set `self.IsLocked` false))

(event `ForceInteractDoor`
  (params (IsOpening :type Boolean))
  (if (`self.IsLocked`)
    _
    (elif (not (`self.IsMoving`))
      (set `self.IsMoving` true)
      (bind _output_get (set `self.IsOpened` IsOpening))
      (if _output_get
        (bind (_direction _door_alpha) (`Timeline|Timeline` :!label _label_2)
          (:`Update`
            (`SceneComponent.K2_SetRelativeRotation` (`self.Door`) (`KismetMathLibrary.MakeRotator` 0.0 0.0 (`KismetMathLibrary.Lerp` 0.0 100.0 _door_alpha)) false false))
          (:`Finished`
            (set `self.IsMoving` false)))
        (else
          (goto _label_2 :!via `ReverseFromEnd`))))))

(event `CustomEvent`
  (params (Doors :type "/Game/TheDawnOffice/Content/Door/BP_Door Object Reference"))
  (set `self.IsLocked` false))

(fn `UserConstructionScript`
  (`parent.UserConstructionScript`))