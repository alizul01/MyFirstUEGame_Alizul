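; BP_Trigger is a box trigger volume that plays a 2D sound when the player character overlaps it, optionally firing a jumpscare.
; With Jumpscare enabled, it calls JumpscareMessage on the referenced Actor before the sound, and does nothing if that reference is invalid.
; With OnlyOnce set, the trigger destroys itself after playing the sound.
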(event `self.Box.OnComponentBeginOverlap`
  (params (OverlappedComponent :type "PrimitiveComponent Object Reference") (OtherActor :type "Actor Object Reference") (OtherComp :type "PrimitiveComponent Object Reference") (OtherBodyIndex :type Integer) (bFromSweep :type Boolean) (SweepResult :type "HitResult Structure (by ref)"))
  (bind _actor (`self.Actor`))
  (if (== OtherActor (`GameplayStatics.GetPlayerCharacter` 0))
    (if (`self.Jumpscare`)
      (`/Engine/EditorBlueprintResources/StandardMacros.IsValid` _actor
        (:`Is Valid`
          (message `/Game/TheDawnOffice/Content/Ghost/BPI_Jumpscare.Jumpscare` _actor))))
    (`GameplayStatics.PlaySound2D` (`self.Sfx`) 1.0 1.0 0.0 null null)
    (if (`self.OnlyOnce?`)
      (`self.K2_DestroyActor`))))

(fn `UserConstructionScript`)