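; Dialogue manager that shows a speaker's lines one at a time and can freeze the first-person player character.
; BeginPlay caches the character and creates the WBP_Dialogue widget.
; Each StartDialogue call sends the next line, speaker name and text delay to the widget; once lines run out it resets the index, clears the screen and unfreezes the player.
; A separate Speech event optionally applies the freeze.
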(event `self.ReceiveBeginPlay`
  (`|ExecutionSequence`
    (:`then_0`
      (bind _asbp_first_person_character (cast `/Game/FirstPerson/Blueprints/BP_FirstPersonCharacter` (`GameplayStatics.GetPlayerCharacter` 0)))
      (set `self.Character` _asbp_first_person_character))
    (:`then_1`
      (bind _returnvalue (`|CreateWidget` "/Game/TheDawnOffice/Widget/WBP_Dialogue.WBP_Dialogue_C"))
      (set `self.W_DialogueRef` _returnvalue))))

(event `Speech`
  (params (`Freeze?` :type Boolean))
  (if `Freeze?`
    (`self.FreezeCharacter` true)))

(fn `FreezeCharacter`
  (params (`Freeze?` :type Boolean))
  (bind _character (`self.Character`))
  (if `Freeze?`
    (`/Game/FirstPerson/Blueprints/BP_FirstPersonCharacter.FreezeCharacter` _character)
    (else
      (`/Game/FirstPerson/Blueprints/BP_FirstPersonCharacter.UnFreezeCharacter` _character))))

(fn `StartDialogue`
  (params (NewParam :type "/Game/TheDawnOffice/Content/Dialogue/Data/BP_DialogueData Object Reference"))
  (bind _currentdialogue (`self.CurrentDialogue`))
  (bind _dialogue (`/Game/TheDawnOffice/Content/Dialogue/Data/BP_DialogueData.Dialogue` (`self.DialogueRef`)))
  (set `self.DialogueRef` NewParam)
  (if (< _currentdialogue (`KismetArrayLibrary.Array_Length` _dialogue))
    (`/Game/TheDawnOffice/Widget/WBP_Dialogue.IncomingText` (`self.W_DialogueRef`) (`|GetArrayItem` _dialogue _currentdialogue) (`self.TextDelay`) (`/Game/TheDawnOffice/Content/Dialogue/Data/BP_DialogueData.Name` (`self.DialogueRef`)))
    (bind _result (`/Engine/EditorBlueprintResources/StandardMacros.IncrementInt` (`self.CurrentDialogue`)))
    (else
      (set `self.CurrentDialogue` 0)
      (`/Game/TheDawnOffice/Widget/WBP_Dialogue.ClearScreen` (`self.W_DialogueRef`))
      (`/Game/FirstPerson/Blueprints/BP_FirstPersonCharacter.UnFreezeCharacter` (`self.Character`)))))

(fn `UserConstructionScript`)