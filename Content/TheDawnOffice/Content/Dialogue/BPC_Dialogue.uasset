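; BPC_Dialogue is an actor component that shows an NPC's named dialogue lines through a WBP_Dialogue widget.
; It creates the widget on BeginPlay.
; Each Speech call pauses the game and sends the current line, speaker name and text delay to the widget, then advances the index.
; Once the lines run out, it resets the index, clears the screen and unpauses.
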(event `self.ReceiveBeginPlay`
  (bind _returnvalue (`|CreateWidget` "/Game/TheDawnOffice/Widget/WBP_Dialogue.WBP_Dialogue_C"))
  (set `self.W_DialogueRef` _returnvalue))

(event `Speech`
  (bind _dialogue (`self.Dialogue`))
  (bind _currentdialogue (`self.CurrentDialogue`))
  (`GameplayStatics.SetGamePaused` true)
  (if (< _currentdialogue (`KismetArrayLibrary.Array_Length` _dialogue))
    (`/Game/TheDawnOffice/Widget/WBP_Dialogue.IncomingText` (`self.W_DialogueRef`) (`|GetArrayItem` _dialogue _currentdialogue) (`self.TextDelay`) (`self.Name`))
    (bind _result (`/Engine/EditorBlueprintResources/StandardMacros.IncrementInt` (`self.CurrentDialogue`)))
    (else
      (set `self.CurrentDialogue` 0)
      (`/Game/TheDawnOffice/Widget/WBP_Dialogue.ClearScreen` (`self.W_DialogueRef`))
      (`GameplayStatics.SetGamePaused` false))))