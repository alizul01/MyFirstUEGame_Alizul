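; BP_SecurityMonitor is an interactable security monitor that hooks into the objective system.
; On BeginPlay it copies its ObjectiveData and ObjectiveDataComplete, when valid, into its BPObjectiveComponent as the objectives to add and to complete.
; The Interact event calls ExecuteObjective on that component, which handles the objective logic.
; The construction script only calls the parent's.
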(event `/Game/TheDawnOffice/Content/Items/Interfaces/I_Interact.Interact`
  (params (Character :type "/Game/FirstPerson/Blueprints/BP_FirstPersonCharacter Object Reference"))
  (`/Game/TheDawnOffice/Content/Objectives/ObjectiveSystem/BP_ObjectiveComponent.ExecuteObjective` (`self.BP_ObjectiveComponent`)))

(event `self.ReceiveBeginPlay`
  (bind _objectivedata (`self.ObjectiveData`))
  (bind _bp_objectivecomponent (`self.BP_ObjectiveComponent`))
  (bind _objectivedatacomplete (`self.ObjectiveDataComplete`))
  (`/Engine/EditorBlueprintResources/StandardMacros.IsValid` _objectivedata
    (:`Is Valid`
      (set `/Game/TheDawnOffice/Content/Objectives/ObjectiveSystem/BP_ObjectiveComponent.ObjectiveToAdd` _objectivedata _bp_objectivecomponent))
    (:`Is Not Valid`
      _))
  (`/Engine/EditorBlueprintResources/StandardMacros.IsValid` _objectivedatacomplete
    (:`Is Valid`
      (set `/Game/TheDawnOffice/Content/Objectives/ObjectiveSystem/BP_ObjectiveComponent.ObjectiveToComplete` _objectivedatacomplete _bp_objectivecomponent))))

(fn `UserConstructionScript`
  (`parent.UserConstructionScript`))