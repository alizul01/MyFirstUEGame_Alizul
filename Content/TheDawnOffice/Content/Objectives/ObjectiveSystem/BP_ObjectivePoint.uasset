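; Objective trigger actor that shows an on-screen objective when the player character enters its box, sized by the construction script.
; It creates a WBP_Objective at BeginPlay, then on first overlap fills in its text, plays a sound, fades it with ObjectiveFade, reverses after a delay and sets ObjectiveInProgress.
; CompleteObjective reuses the widget to show "Objective Completed" with the same sound, replaying the fade forward both times.
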(event `self.ReceiveBeginPlay`
  (bind _returnvalue (`|CreateWidget` "/Game/TheDawnOffice/Widget/WBP_Objective.WBP_Objective_C" null (`self.ObjectiveTitleText`) (`self.ObjectiveContentText`)))
  (set `self.WBP_ObjectiveWidgetRef` _returnvalue))

(event `self.ObjectiveBox.OnComponentBeginOverlap`
  (params (OverlappedComponent :type "PrimitiveComponent Object Reference") (OtherActor :type "Actor Object Reference") (OtherComp :type "PrimitiveComponent Object Reference") (OtherBodyIndex :type Integer) (bFromSweep :type Boolean) (SweepResult :type "HitResult Structure (by ref)"))
  (bind _wbp_objectivewidgetref (`self.WBP_ObjectiveWidgetRef`))
  (bind _wbp_objectivewidgetref_2 (`self.WBP_ObjectiveWidgetRef`))
  (bind _objectivefade (`/Game/TheDawnOffice/Widget/WBP_Objective.ObjectiveFade` _wbp_objectivewidgetref_2))
  (if (== OtherActor (`GameplayStatics.GetPlayerCharacter` 0))
    (`/Engine/EditorBlueprintResources/StandardMacros.DoOnce` false
      (:`Completed`
        (set `/Game/TheDawnOffice/Widget/WBP_Objective.ObjectiveTitleText` (`self.ObjectiveTitleText`) _wbp_objectivewidgetref)
        (set `/Game/TheDawnOffice/Widget/WBP_Objective.ObjectiveContentText` (`self.ObjectiveContentText`) _wbp_objectivewidgetref)
        (`TextBlock.SetColorAndOpacity` (`/Game/TheDawnOffice/Widget/WBP_Objective.ObjectiveContent` _wbp_objectivewidgetref) (make `SlateColor` (make `LinearColor` 1.0 1.0 1.0 0.5)))
        (`GameplayStatics.PlaySound2D` "/Game/TheDawnOffice/SoundsOfHorror/Clues/WAVE/WAV_SOH_Clue_06.WAV_SOH_Clue_06" 1.0 1.0 0.0 null null)
        (`UserWidget.AddToViewport` _wbp_objectivewidgetref_2 0)
        (`UserWidget.PlayAnimation` _wbp_objectivewidgetref_2 _objectivefade 0.0 1 "Forward" 1.0 false)
        (`KismetSystemLibrary.Delay` 5.0)
        (`UserWidget.PlayAnimation` _wbp_objectivewidgetref_2 _objectivefade 0.0 1 "Reverse" 1.0 false)
        (set `self.ObjectiveInProgress?` true)))))

(event `Complete Objective`
  (bind _wbp_objectivewidgetref (`self.WBP_ObjectiveWidgetRef`))
  (bind _objectivefade (`/Game/TheDawnOffice/Widget/WBP_Objective.ObjectiveFade` _wbp_objectivewidgetref))
  (set `/Game/TheDawnOffice/Widget/WBP_Objective.ObjectiveTitleText` "Objective Completed" _wbp_objectivewidgetref)
  (`TextBlock.SetColorAndOpacity` (`/Game/TheDawnOffice/Widget/WBP_Objective.ObjectiveContent` _wbp_objectivewidgetref) (make `SlateColor` (make `LinearColor` 1.0 1.0 1.0 0.5)))
  (`GameplayStatics.PlaySound2D` "/Game/TheDawnOffice/SoundsOfHorror/Clues/WAVE/WAV_SOH_Clue_06.WAV_SOH_Clue_06" 1.0 1.0 0.0 null null)
  (`UserWidget.PlayAnimation` _wbp_objectivewidgetref _objectivefade 0.0 1 "Forward" 1.0 false)
  (`KismetSystemLibrary.Delay` 3.0)
  (`UserWidget.PlayAnimation` (`self.WBP_ObjectiveWidgetRef`) _objectivefade 0.0 1 "Forward" 1.0 false))

(fn `UserConstructionScript`
  (`BoxComponent.SetBoxExtent` (`self.ObjectiveBox`) (`self.ObjectiveBoxSize`) true))