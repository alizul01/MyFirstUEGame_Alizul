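; Objective manager that tracks active and completed player objectives and displays them in an on-screen HUD list.
; UpdateObjectiveProgress routes an action type to add, complete, or complete-then-add, using a map of objective to progress count.
; Completing increments the count, moving objectives that reach their target to the completed list.
; Changes rebuild the HUD with animated row widgets, showing counters for multi-step objectives, and play sound cues.
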(event `self.ReceiveBeginPlay`
  (bind _returnvalue (`|CreateWidget` "/Game/TheDawnOffice/Content/Objectives/Widget/WBP_ObjectiveHUD.WBP_ObjectiveHUD_C"))
  (set `self.HUD_Reference` _returnvalue))

(fn `AddObjective`
  (params (Key :type "/Game/TheDawnOffice/Content/Objectives/ObjectiveData/BP_ObjectiveData Object Reference (by ref)"))
  (`BlueprintMapLibrary.Map_Add` (`self.ActiveObjectivesProgress`) Key)
  (`self.ShowUI`))

(fn `CompleteObjective`
  (params (Key :type "/Game/TheDawnOffice/Content/Objectives/ObjectiveData/BP_ObjectiveData Object Reference"))
  (locals (ObjData :type "/Game/TheDawnOffice/Content/Objectives/ObjectiveData/BP_ObjectiveData Object Reference"))
  (bind _objdata (`local.ObjData`))
  (bind _output_get (set `local.ObjData` Key))
  (bind (_value _returnvalue) (`BlueprintMapLibrary.Map_Find` (`self.ActiveObjectivesProgress`) _output_get))
  (if _returnvalue
    (`KismetSystemLibrary.PrintString` (`KismetTextLibrary.Conv_TextToString` (`|FormatText` "Current Value: {current}" (`KismetStringLibrary.Conv_IntToString` _value))) true true (struct :`G` 0.66 :`B` 1.0 :`A` 1.0) 10.0)
    (bind _returnvalue_2 (+ _value 1))
    (`BlueprintMapLibrary.Map_Add` (`self.ActiveObjectivesProgress`) (`local.ObjData`) _returnvalue_2)
    (if (>= _returnvalue_2 (`/Game/TheDawnOffice/Content/Objectives/ObjectiveData/BP_ObjectiveData.TargetCount` (`local.ObjData`)))
      (`BlueprintMapLibrary.Map_Remove` (`self.ActiveObjectivesProgress`) _objdata)
      (`KismetArrayLibrary.Array_AddUnique` (`self.CompletedObjectives`) _objdata)
      (`GameplayStatics.PlaySound2D` "/Engine/EditorSounds/Notifications/CompileSuccess.CompileSuccess" 1.0 1.0 0.0 null null)
      (`self.ShowUI`)
      (else
        (`GameplayStatics.PlaySound2D` "/Engine/EditorSounds/Notifications/CompileFailed.CompileFailed" 1.0 1.0 0.0 null null)
        (`self.ShowUI`)))))

(fn `ShowUI`
  (locals (L_FinalText :type Text))
  (bind _hud_reference (`self.HUD_Reference`))
  (`/Engine/EditorBlueprintResources/StandardMacros.IsValid` _hud_reference
    (:`Is Valid`
      (`PanelWidget.ClearChildren` (`/Game/TheDawnOffice/Content/Objectives/Widget/WBP_ObjectiveHUD.ObjectiveList_Container` _hud_reference))
      (bind _keys (`BlueprintMapLibrary.Map_Keys` (`self.ActiveObjectivesProgress`)))
      (for _array_element _keys
        (bind _targetcount (`/Game/TheDawnOffice/Content/Objectives/ObjectiveData/BP_ObjectiveData.TargetCount` _array_element))
        (if (> _targetcount 1)
          (bind _title (`/Game/TheDawnOffice/Content/Objectives/ObjectiveData/BP_ObjectiveData.Title` _array_element))
          (set `local.L_FinalText` (`|FormatText` "{Title} ({Current}/{Max})" _title (`BlueprintMapLibrary.Map_Find` (`self.ActiveObjectivesProgress`) _array_element) _targetcount))
          (else
            (set `local.L_FinalText` _title)))
        (bind _returnvalue (`|CreateWidget` "/Game/TheDawnOffice/Content/Objectives/Widget/WBP_ObjectiveRow.WBP_ObjectiveRow_C" null (`local.L_FinalText`)))
        (`VerticalBox.AddChildToVerticalBox` (`/Game/TheDawnOffice/Content/Objectives/Widget/WBP_ObjectiveHUD.ObjectiveList_Container` (`self.HUD_Reference`)) _returnvalue)
        (`UserWidget.AddToViewport` (`self.HUD_Reference`) 0)
        (`GameplayStatics.PlaySound2D` "/Game/TheDawnOffice/SoundsOfHorror/Clues/WAVE/WAV_SOH_Clue_06.WAV_SOH_Clue_06" 1.0 1.0 0.0 null null)
        (`Widget.SetRenderOpacity` (`/Game/TheDawnOffice/Content/Objectives/Widget/WBP_ObjectiveRow.HorizontalBox_243` _returnvalue) 0.0)
        (`UserWidget.PlayAnimation` _returnvalue (`/Game/TheDawnOffice/Content/Objectives/Widget/WBP_ObjectiveRow.AnimIn` _returnvalue) 0.0 1 "Forward" 1.0 false)))))

(fn `UpdateObjectiveProgress`
  (params (ObjectiveData :type "/Game/TheDawnOffice/Content/Objectives/ObjectiveData/BP_ObjectiveData Object Reference") (ActionType :type "/Game/TheDawnOffice/Content/Objectives/ObjectiveSystem/E_ObjectiveAction Enum" :default "NewEnumerator0") (ObjectiveToComplete :type "/Game/TheDawnOffice/Content/Objectives/ObjectiveData/BP_ObjectiveData Object Reference"))
  (locals (ObjectiveToAdd :type "/Game/TheDawnOffice/Content/Objectives/ObjectiveData/BP_ObjectiveData Object Reference"))
  (set `local.ObjectiveToAdd` ObjectiveData)
  (switch `/Game/TheDawnOffice/Content/Objectives/ObjectiveSystem/E_ObjectiveAction` ActionType
    (:`NewEnumerator0`
      (`self.AddObjective` (`local.ObjectiveToAdd`)))
    (:`NewEnumerator1`
      (`self.CompleteObjective` ObjectiveToComplete))
    (:`NewEnumerator2`
      (`self.CompleteObjective` ObjectiveToComplete)
      (`self.AddObjective` (`local.ObjectiveToAdd`)))))

(fn `UserConstructionScript`)