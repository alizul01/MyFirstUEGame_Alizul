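; BP_ObjectiveTrigger is a trigger actor that reports progress on a target objective to the objective system.
; Depending on TriggerType, it fires from the first-person character overlapping its box, an Interact event, or an external CallByEvent.
; All three paths share ExecuteObjective, which passes a DoOnce fed by IsOneShot, then finds BP_ObjectiveManager and calls UpdateObjectiveProgress with the objective and action type.
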(event `ExecuteObjective`
  (`/Engine/EditorBlueprintResources/StandardMacros.DoOnce` (`self.IsOneShot`)
    (:`Completed`
      (bind _returnvalue (`GameplayStatics.GetActorOfClass` "/Game/TheDawnOffice/Content/Objectives/ObjectiveSystem/BP_ObjectiveManager.BP_ObjectiveManager_C"))
      (`/Game/TheDawnOffice/Content/Objectives/ObjectiveSystem/BP_ObjectiveManager.UpdateObjectiveProgress` _returnvalue (`self.TargetObjective`) (`self.Type`) null))))

(event `self.Box.OnComponentBeginOverlap`
  (params (OverlappedComponent :type "PrimitiveComponent Object Reference") (OtherActor :type "Actor Object Reference") (OtherComp :type "PrimitiveComponent Object Reference") (OtherBodyIndex :type Integer) (bFromSweep :type Boolean) (SweepResult :type "HitResult Structure (by ref)"))
  (cast `/Game/FirstPerson/Blueprints/BP_FirstPersonCharacter` OtherActor)
  (switch `/Game/TheDawnOffice/Content/Objectives/ObjectiveSystem/E_TriggerType` (`self.TriggerType`)
    (:`NewEnumerator0`
      (`self.ExecuteObjective`))))

(event `/Game/TheDawnOffice/Content/Items/Interfaces/I_Interact.Interact`
  (params (Character :type "/Game/FirstPerson/Blueprints/BP_FirstPersonCharacter Object Reference"))
  (switch `/Game/TheDawnOffice/Content/Objectives/ObjectiveSystem/E_TriggerType` (`self.TriggerType`)
    (:`NewEnumerator1`
      (`self.ExecuteObjective`))))

(event `CallByEvent`
  (switch `/Game/TheDawnOffice/Content/Objectives/ObjectiveSystem/E_TriggerType` (`self.TriggerType`)
    (:`NewEnumerator2`
      (`self.ExecuteObjective`))))

(fn `UserConstructionScript`)