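; BP_Interactable is a world item that shows proximity prompts and can open an inspection view when the player interacts with it.
; Inner and outer spheres, sized in the construction script, switch between far and near interact icons for the player character.
; If inspectable, Interact spawns a BP_InspectionItem far outside the level, passing it the mesh, display transform, name, description, type, pickup flag and itself.
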(event `/Game/TheDawnOffice/Content/Items/Interfaces/I_Interact.Interact`
  (params (Character :type "/Game/FirstPerson/Blueprints/BP_FirstPersonCharacter Object Reference"))
  (if (`self.IsInspectable`)
    (bind _returnvalue (`|SpawnActorFromClass` "/Game/TheDawnOffice/Content/Items/BP_InspectionItem.BP_InspectionItem_C" (`KismetMathLibrary.MakeTransform` (10000000000.0 0.0 0.0)) "Undefined" "MultiplyWithRoot" null null))
    (`/Game/TheDawnOffice/Content/Items/BP_InspectionItem.Set Item Rotation` _returnvalue (`self.InspectItemRotation`))
    (`/Game/TheDawnOffice/Content/Items/BP_InspectionItem.Set Item Scale` _returnvalue (`self.InspectItemScale`))
    (`/Game/TheDawnOffice/Content/Items/Interfaces/I_Interact.Inspect` _returnvalue Character (`StaticMeshComponent.StaticMesh` (`self.StaticMesh`)) (`self.Item Name`) (`self.Item Description`) (`self.IsPickupable`) self (`self.Item Type`))))

(event `self.InnerSphereCollision.OnComponentBeginOverlap`
  (params (OverlappedComponent :type "PrimitiveComponent Object Reference") (OtherActor :type "Actor Object Reference") (OtherComp :type "PrimitiveComponent Object Reference") (OtherBodyIndex :type Integer) (bFromSweep :type Boolean) (SweepResult :type "HitResult Structure (by ref)"))
  (if (== OtherActor (`GameplayStatics.GetPlayerCharacter` 0))
    (`SceneComponent.SetVisibility` (`self.InnerInteractIcon`) true false)
    (`SceneComponent.SetVisibility` (`self.OuterInteractIcon`) false false)))

(event `self.InnerSphereCollision.OnComponentEndOverlap`
  (params (OverlappedComponent :type "PrimitiveComponent Object Reference") (OtherActor :type "Actor Object Reference") (OtherComp :type "PrimitiveComponent Object Reference") (OtherBodyIndex :type Integer))
  (if (== OtherActor (`GameplayStatics.GetPlayerCharacter` 0))
    (`SceneComponent.SetVisibility` (`self.InnerInteractIcon`) false false)
    (`SceneComponent.SetVisibility` (`self.OuterInteractIcon`) true false)))

(event `self.OuterSphereCollision.OnComponentBeginOverlap`
  (params (OverlappedComponent :type "PrimitiveComponent Object Reference") (OtherActor :type "Actor Object Reference") (OtherComp :type "PrimitiveComponent Object Reference") (OtherBodyIndex :type Integer) (bFromSweep :type Boolean) (SweepResult :type "HitResult Structure (by ref)"))
  (if (== OtherActor (`GameplayStatics.GetPlayerCharacter` 0))
    (`SceneComponent.SetVisibility` (`self.OuterInteractIcon`) true false)))

(event `self.OuterSphereCollision.OnComponentEndOverlap`
  (params (OverlappedComponent :type "PrimitiveComponent Object Reference") (OtherActor :type "Actor Object Reference") (OtherComp :type "PrimitiveComponent Object Reference") (OtherBodyIndex :type Integer))
  (if (== (`GameplayStatics.GetPlayerCharacter` 0) OtherActor)
    (`SceneComponent.SetVisibility` (`self.OuterInteractIcon`) false false)))

(fn `UserConstructionScript`
  (`SphereComponent.SetSphereRadius` (`self.InnerSphereCollision`) (`self.InnerSphereRadius`) true)
  (`SphereComponent.SetSphereRadius` (`self.OuterSphereCollision`) (`self.OuterSphereRadius`) true))