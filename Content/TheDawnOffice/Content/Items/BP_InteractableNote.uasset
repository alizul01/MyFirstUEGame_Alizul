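; Interactable note item that the player reads as an on-screen WBP_Note widget.
; Interact toggles via FlipFlop between showing the widget with movement and look input locked, and removing it to restore both.
; Opening also calls Read and, if IsAddNewObjective is set, executes the objective component.
; Inner and outer spheres, sized in the construction script, swap near and far interaction icons as the player overlaps them.
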(event `self.Interact`
  (params (Character :type "/Game/FirstPerson/Blueprints/BP_FirstPersonCharacter Object Reference"))
  (bind _returnvalue (`GameplayStatics.GetPlayerController` 0))
  (bind _charactermovement (`Character.CharacterMovement` (`GameplayStatics.GetPlayerCharacter` 0)))
  (bind _isa (`/Engine/EditorBlueprintResources/StandardMacros.FlipFlop`)
    (:`A`
      (set `self.Is A` _isa)
      (bind _returnvalue_2 (`|CreateWidget` "/Game/TheDawnOffice/Widget/WBP_Note.WBP_Note_C" null (`self.NoteText`) (`self.Item Name`) (`self.Item Description`)))
      (bind _output_get (set `self.NoteWidget` _returnvalue_2))
      (`UserWidget.AddToViewport` _output_get 0)
      (`CharacterMovementComponent.DisableMovement` (`Character.CharacterMovement` (`GameplayStatics.GetPlayerCharacter` 0)))
      (`Controller.SetIgnoreLookInput` _returnvalue true)
      (`Widget.SetRenderOpacity` (`/Game/TheDawnOffice/Widget/WBP_Note.NoteCanvasPanel` (`self.NoteWidget`)) 1.0)
      (set `self.Is A` false)
      (`/Game/TheDawnOffice/Content/Items/Interfaces/I_Interact.Read` Character (`self.NoteText`))
      (if (`self.IsAddNewObjective?`)
        (`/Game/TheDawnOffice/Content/Objectives/ObjectiveSystem/BP_ObjectiveComponent.ExecuteObjective` (`self.BP_ObjectiveComponent`))))
    (:`B`
      (`Widget.SetRenderOpacity` (`/Game/TheDawnOffice/Widget/WBP_Note.NoteCanvasPanel` (`self.NoteWidget`)) 1.0)
      (`Widget.RemoveFromParent` _returnvalue_2)
      (`CharacterMovementComponent.SetMovementMode` _charactermovement (`CharacterMovementComponent.DefaultLandMovementMode` _charactermovement) 0)
      (`Controller.SetIgnoreLookInput` _returnvalue false)
      (set `self.Is A` true))))

(event `self.InnerSphereCollision.OnComponentBeginOverlap`
  (params (OverlappedComponent :type "PrimitiveComponent Object Reference") (OtherActor :type "Actor Object Reference") (OtherComp :type "PrimitiveComponent Object Reference") (OtherBodyIndex :type Integer) (bFromSweep :type Boolean) (SweepResult :type "HitResult Structure (by ref)"))
  (if (== OtherActor (`GameplayStatics.GetPlayerCharacter` 0))
    (`SceneComponent.SetVisibility` (`self.InnerInteractIcon`) true false)
    (`SceneComponent.SetVisibility` (`self.OuterInteractIcon`) false false)))

(event `self.InnerSphereCollision.OnComponentEndOverlap`
  (params (OverlappedComponent :type "PrimitiveComponent Object Reference") (OtherActor :type "Actor Object Reference") (OtherComp :type "PrimitiveComponent Object Reference") (OtherBodyIndex :type Integer))
  (if (== OtherActor (`GameplayStatics.GetPlayerCharacter` 0))
    (`SceneComponent.SetVisibility` (`self.InnerInteractIcon`) false false)
    (`SceneComponent.SetVisibility` (`self.OuterInteractIcon`) true false)))

(event `self.OuterSphereCollision.OnComponentBeginOverlap`
  (params (OverlappedComponent :type "PrimitiveComponent Object Reference") (OtherActor :type "Actor Object Reference") (OtherComp :type "PrimitiveComponent Object Reference") (OtherBodyIndex :type Integer) (bFromSweep :type Boolean) (SweepResult :type "HitResult Structure (by ref)"))
  (if (== OtherActor (`GameplayStatics.GetPlayerCharacter` 0))
    (`SceneComponent.SetVisibility` (`self.OuterInteractIcon`) true false)))

(event `self.OuterSphereCollision.OnComponentEndOverlap`
  (params (OverlappedComponent :type "PrimitiveComponent Object Reference") (OtherActor :type "Actor Object Reference") (OtherComp :type "PrimitiveComponent Object Reference") (OtherBodyIndex :type Integer))
  (if (== (`GameplayStatics.GetPlayerCharacter` 0) OtherActor)
    (`SceneComponent.SetVisibility` (`self.OuterInteractIcon`) false false)))

(fn `UserConstructionScript`
  (`SphereComponent.SetSphereRadius` (`self.InnerSphereCollision`) (`self.InnerSphereRadius`) true)
  (`SphereComponent.SetSphereRadius` (`self.OuterSphereCollision`) (`self.OuterSphereRadius`) true))