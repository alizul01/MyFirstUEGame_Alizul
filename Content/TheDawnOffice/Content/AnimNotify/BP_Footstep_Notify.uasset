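; Animation notify that plays brick or concrete footstep sounds for player character 0, whichever mesh fires it.
; A short downward Visibility trace finds the surface type and selects the cue, defaulting to concrete, to play at the hit point.
; Player speed sets run or walk volume; slow movement is silent, as the crouch-volume sound is never reached.
; The returned surface number only feeds checks that return true.
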(fn `GetSurface`
  (returns (Surface :type "Float (double-precision)"))
  (locals (SurfaceParameter :type "Float (double-precision)"))
  (bind _returnvalue (`Actor.K2_GetActorLocation` (`GameplayStatics.GetPlayerCharacter` 0)))
  (bind (_outhit _returnvalue_2) (`KismetSystemLibrary.LineTraceSingle` _returnvalue (- _returnvalue (0.0 0.0 150.0)) "TraceTypeQuery1"))
  (if _returnvalue_2
    (switch `EPhysicalSurface` (`GameplayStatics.GetSurfaceType` _outhit)
      (:`SurfaceType_Default`
        (set `local.SurfaceParameter` 1.0)
        (bind (_bblockinghit _binitialoverlap _time _distance _location) (`GameplayStatics.BreakHitResult` _outhit))
        (`self.PlaySoundAtLocaiton` "/Game/TheDawnOffice/Arts/Audio/Sfx/Footstep/Concrete/Cue_Concrete_Footstep.Cue_Concrete_Footstep" _location))
      (:`SurfaceType1`
        (set `local.SurfaceParameter` 3.0)
        (`self.PlaySoundAtLocaiton` "/Game/TheDawnOffice/Arts/Audio/Sfx/Footstep/Concrete/Cue_Concrete_Footstep.Cue_Concrete_Footstep" _location))
      (:`SurfaceType2`
        (set `local.SurfaceParameter` 2.0)
        (`self.PlaySoundAtLocaiton` "/Game/TheDawnOffice/Arts/Audio/Sfx/Footstep/Wood/Cue_Brick_Footstep.Cue_Brick_Footstep" _location)))
    (return (`local.SurfaceParameter`))))

(fn `PlaySoundAtLocaiton`
  (params (Sound :type "SoundBase Object Reference") (Location :type "Vector Structure"))
  (locals (RunVolume :type "Float (single-precision)" :default 2.0) (WalkVolume :type "Float (single-precision)" :default 1.0) (CrouchVolume :type "Float (single-precision)" :default 0.7))
  (bind _returnvalue (`KismetMathLibrary.VSize` (`MovementComponent.Velocity` (`Character.CharacterMovement` (`GameplayStatics.GetPlayerCharacter` 0)))))
  (if (> _returnvalue 230.0)
    (`GameplayStatics.PlaySoundAtLocation` (`local.Sound`) (`local.Location`) (struct) (`local.RunVolume`) 1.0 0.0 null null null null)
    (elif (not (<= _returnvalue 110.0))
      (`GameplayStatics.PlaySoundAtLocation` (`local.Sound`) (`local.Location`) (struct) (`local.WalkVolume`) 1.0 0.0 null null null null))))

(fn `Received_Notify`
  (params (MeshComp :type "SkeletalMeshComponent Object Reference") (Animation :type "AnimSequenceBase Object Reference") (EventReference :type "AnimNotifyEventReference Structure (by ref)"))
  (returns (ReturnValue :type Boolean))
  (locals (`Surface Type Num` :type "Float (double-precision)"))
  (`/Engine/EditorBlueprintResources/StandardMacros.IsValid` MeshComp
    (:`Is Valid`
      (bind _surface (`self.GetSurface`))
      (bind _output_get (set `local.Surface Type Num` _surface))
      (`|ExecutionSequence`
        (:`then_0`
          ; Brick
          (if (== _output_get 3.0)
            (return true)))
        (:`then_1`
          ; Concrete
          (if (== _output_get 2.0)
            (return true)))))
    (:`Is Not Valid`
      (return true))))