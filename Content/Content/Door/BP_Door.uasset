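; Interactable door that cycles through closed, partially open and open on successive interactions.
; Interact picks the swing side from a dot product of player and DoorLookLocation forward vectors, then blocks further interaction until a timer ends.
; Meanwhile, Tick interpolates the door's relative yaw toward the next state's angle with FInterpTo.
; The timer, set by DoorSoundTime, stops the motion and advances the state enum.
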(event `HandleRotation`
  (params (`Set Rotation` :type "Float (double-precision)"))
  ;[0.07664 0.15 0.07049 0.5] Handle Rotation
  (`SceneComponent.K2_SetRelativeRotation` (`self.Door`) (`KismetMathLibrary.MakeRotator` 0.0 0.0 (`KismetMathLibrary.FInterpTo` (.yaw (`SceneComponent.RelativeRotation` (`self.Door`))) `Set Rotation` (`GameplayStatics.GetWorldDeltaSeconds`) (`self.Interp Speed`))) false false))

(event `self.ReceiveBeginPlay`
  (bind _asbp_first_person_character (cast `/Game/FirstPerson/Blueprints/BP_FirstPersonCharacter` (`GameplayStatics.GetPlayerCharacter` 0)))
  (set `self.CharacterRef` _asbp_first_person_character))

(event `self.ReceiveTick`
  (params (DeltaSeconds :type "Float (single-precision)"))
  (if (`self.bIsInteractingWithDoor`)
    (`self.HandleDoor`)))

(event `IsInteractingWithDoor`
  (params (Player :type "/Game/FirstPerson/Blueprints/BP_FirstPersonCharacter Object Reference"))
  ;[0.15 0.1249 0.06646 0.5] Door Interaction Algorithm
  (if (> (`KismetMathLibrary.Dot_VectorVector` (`self.GetActorForwardVector` Player) (`SceneComponent.GetForwardVector` (`self.DoorLookLocation`))) 0.0)
    (set `self.DoorOpenSide` 1.0)
    (else
      (set `self.DoorOpenSide` -1.0)))
  (set `self.bIsInteractingWithDoor` true)
  (`KismetSystemLibrary.K2_SetTimerDelegate` (delegate `CustomEvent`) (`self.DoorSoundTime`)))

(event `/Game/Content/Items/Interfaces/I_Interact.Interact`
  (if (not (`self.bIsInteractingWithDoor`))
    (`self.IsInteractingWithDoor` self (`self.CharacterRef`))))

(event `HandleDoor`
  ;[0.15 0.07132 0.1097 0.5] Handle Door
  (switch `/Game/Content/Door/E_DoorStates` (`self.EDoorStates`)
    (:`NewEnumerator0`
      (`self.HandleRotation` (* 15.0 (`self.DoorOpenSide`))))
    (:`NewEnumerator1`
      (`self.HandleRotation` (* (`self.Door Open Angle`) (`self.DoorOpenSide`))))
    (:`NewEnumerator2`
      (`self.HandleRotation` 0.0))))

(event `CustomEvent`
  ;[0.15 0.1249 0.06646 0.5] Door Interaction Algorithm
  (set `self.bIsInteractingWithDoor` false)
  (switch `/Game/Content/Door/E_DoorStates` (`self.EDoorStates`)
    (:`NewEnumerator0`
      (set `self.EDoorStates` "NewEnumerator1"))
    (:`NewEnumerator1`
      (set `self.EDoorStates` "NewEnumerator2"))
    (:`NewEnumerator2`
      (set `self.EDoorStates` "NewEnumerator0"))))

(fn `UserConstructionScript`
  (`parent.UserConstructionScript`))